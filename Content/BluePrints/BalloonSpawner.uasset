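; Balloon spawner actor that periodically creates balloons at random points inside its SpawnZone box.
; A Tick countdown spawns each balloon, then assigns a yellow, red, green or blue configuration by weighted random roll, with blue most common.
; Each successful spawn also raises the spawner by a growing Z offset, stopping once that offset exceeds MaxMovement.
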(event `self.ReceiveBeginPlay`
  (set `self.TimeBetweenBalloons` (`self.InitialSpawnRate`)))

(event `self.ReceiveTick`
  (params (DeltaSeconds :type "Float (single-precision)"))
  (bind _output_get (set `self.TimeBetweenBalloons` (- (`self.TimeBetweenBalloons`) DeltaSeconds)))
  (if (< _output_get 0.0)
    (bind _spawnedballoon (`self.SpawnBalloon`))
    (`/Engine/EditorBlueprintResources/StandardMacros.IsValid` _spawnedballoon
      (:`Is Valid`
        (`self.SetBalloonConfiguration` _spawnedballoon)
        (`self.IncreaseSpawnerHeight` DeltaSeconds))
      (:`Is Not Valid`
        (`KismetSystemLibrary.PrintString` "Spawn Not Valid")))
    (set `self.TimeBetweenBalloons` (`self.InitialSpawnRate`))))

(fn `IncreaseSpawnerHeight`
  (params (DeltaSeconds :type "Float (double-precision)"))
  (bind _float_movement_amount (`self.Float Movement Amount`))
  (if (not (> _float_movement_amount (`self.MaxMovement`)))
    (bind _output_get (set `self.Float Movement Amount` (+ _float_movement_amount (* 10.0 DeltaSeconds))))
    (`self.K2_AddActorWorldOffset` (`KismetMathLibrary.MakeVector` 0.0 0.0 _output_get))))

(fn `SetBalloonConfiguration`
  (params (Balloon :type "/Game/BluePrints/Balloon Object Reference"))
  (locals (BallonToConfigure :type "/Game/BluePrints/Balloon Object Reference"))
  (set `local.BallonToConfigure` Balloon)
  (bind _output_get (set `self.Random Balloon Selection` (`KismetMathLibrary.RandomInteger` 1000)))
  (if (> _output_get 950)
    (`/Game/BluePrints/Balloon.Set Configuration` (`local.BallonToConfigure`) (`self.Yellow Config`))
    (elif (> _output_get 700)
      (`/Game/BluePrints/Balloon.Set Configuration` (`local.BallonToConfigure`) (`self.Red Config`))
      (elif (> _output_get 650)
        (`/Game/BluePrints/Balloon.Set Configuration` (`local.BallonToConfigure`) (`self.Green Config`))
        (else
          (`/Game/BluePrints/Balloon.Set Configuration` (`local.BallonToConfigure`) (`self.Blue Config`)))))))

(fn `SpawnBalloon`
  (returns (SpawnedBalloon :type "/Game/BluePrints/Balloon Object Reference"))
  (bind _returnvalue (`|SpawnActorFromClass` "/Game/BluePrints/Balloon.Balloon_C" (`KismetMathLibrary.Conv_VectorToTransform` (`KismetMathLibrary.RandomPointInBoundingBox` (`SceneComponent.K2_GetComponentLocation` (`self.SpawnZone`)) (`BoxComponent.GetScaledBoxExtent` (`self.SpawnZone`)))) "Undefined" "OverrideRootScale" null null))
  (return _returnvalue))

(fn `UserConstructionScript`)