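; First-person player character for a balloon-bouncing score game, with double jump, pistol, pause menu and fall respawn.
; Landing on a balloon adds score and relaunches the player; any other landing submits the high score, saves and resets.
; Shooting and landing switch between three music tracks by score tier.
; The two lower tiers start from a shared looping timer to stay in sync, while the top tier restarts.
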(event `self.ReceiveBeginPlay`
  (bind _asballoon_game_instance (cast `/Game/BluePrints/BalloonGameInstance` (`GameplayStatics.GetGameInstance`)))
  (set `self.Game Instance` _asballoon_game_instance)
  (`self.SetUpWeapon`)
  (`self.SetUpUI`)
  (set `self.Respawn Location` (`self.K2_GetActorLocation`))
  (`self.SetUpAudio`))

(event `self.ReceiveTick`
  (params (DeltaSeconds :type "Float (single-precision)"))
  (bind (_returnvalue_x _returnvalue_y _returnvalue_z) (`KismetMathLibrary.BreakVector` (`self.K2_GetActorLocation`)))
  (bind _output_get (set `self.Song Start` (+ DeltaSeconds (`self.Song Start`))))
  (if (> _output_get 120.0)
    (set `self.Song Start` 0.0))
  (if (> -60.0 _returnvalue_z)
    (`self.K2_SetActorLocation` (`self.Respawn Location`))))

(event `InputAxis|MoveForward`
  (params (AxisValue :type "Float (single-precision)"))
  (`self.AddMovementInput` (`self.GetActorForwardVector`) (* AxisValue 1000.0)))

(event `InputAxis|MoveRight`
  (params (AxisValue :type "Float (single-precision)"))
  (`self.AddMovementInput` (`self.GetActorRightVector`) (* AxisValue 1000.0)))

(event `InputAxis|LookHorizontal`
  (params (AxisValue :type "Float (single-precision)"))
  (`self.AddControllerYawInput` (* AxisValue 1.0)))

(event `InputAxis|LookVertical`
  (params (AxisValue :type "Float (single-precision)"))
  (`self.AddControllerPitchInput` (* AxisValue -1.0)))

(event `InputAction|Jump`
  (params (Key :type "Key Structure"))
  (:`Pressed`
    (if (`NavMovementComponent.IsFalling` (`self.CharacterMovement`))
      (if (`self.CanDoubleJump`)
        (set `self.CanDoubleJump` false)
        (`self.Launch Player` (`self.Jump Height`) :!label _label))
      (else
        (set `/Game/UI/Score_HUD.CanScore` true (`self.UI Reference`))
        (goto _label)))))

(event `InputAction|Shoot`
  (params (Key :type "Key Structure"))
  (bind _fpscamera (`self.FpsCamera`))
  (:`Pressed`
    (`/Game/BluePrints/BP_BaseGun.Shoot` (`self.EquippedGun`) (`SceneComponent.K2_GetComponentLocation` _fpscamera) (`SceneComponent.GetForwardVector` _fpscamera))
    (`self.MusicUpdate` (`/Game/UI/Score_HUD.Score` (`self.UI Reference`)))))

(event `self.OnLanded`
  (params (Hit :type "HitResult Structure (by ref)"))
  (bind _ui_reference (`self.UI Reference`))
  (bind _game_instance (`self.Game Instance`))
  (set `self.CanDoubleJump` true)
  (bind _asballoon (cast `/Game/BluePrints/Balloon` (`.HitActor` (`GameplayStatics.BreakHitResult` Hit)))
    (:`then`
      (bind (_scorevalue _jumpamount) (`/Game/BluePrints/Balloon.JumpedOn` _asballoon))
      (`/Game/UI/Score_HUD.AddToScore` (`self.UI Reference`) _scorevalue)
      (`self.Launch Player` _jumpamount))
    (:`CastFailed`
      (`/Game/BluePrints/BalloonGameInstance.AttemptToSetHighScore` _game_instance (`/Game/UI/Score_HUD.Score` (`self.UI Reference`)))
      (`/Game/UI/Score_HUD.ResetScore` _ui_reference)
      (`/Game/UI/Score_HUD.SetCanScore` _ui_reference false)
      (`/Game/BluePrints/BalloonGameInstance.Save Game` _game_instance)))
  (`self.MusicUpdate` (`/Game/UI/Score_HUD.Score` (`self.UI Reference`))))

(event `InputAction|Pause` :paused true
  (params (Key :type "Key Structure"))
  (bind _returnvalue (`GameplayStatics.GetPlayerController` 0))
  (:`Pressed`
    (if (`GameplayStatics.IsGamePaused`)
      (`Widget.SetVisibility` (`self.Pause Menu`) "Hidden")
      (`WidgetBlueprintLibrary.SetInputMode_GameOnly` _returnvalue)
      (set `PlayerController.bShowMouseCursor` false _returnvalue)
      (`GameplayStatics.SetGamePaused` false)
      (else
        (`Widget.SetVisibility` (`self.Pause Menu`) "Visible")
        (`GameplayStatics.SetGamePaused` true)
        (`WidgetBlueprintLibrary.SetInputMode_GameAndUIEx` _returnvalue null)
        (set `PlayerController.bShowMouseCursor` true _returnvalue)))))

(fn `Launch Player`
  (params (Amount :type "Float (double-precision)"))
  (bind _charactermovement (`self.CharacterMovement`))
  (bind (_velocity_x _velocity_y) (`KismetMathLibrary.BreakVector` (`MovementComponent.Velocity` _charactermovement)))
  (set `MovementComponent.Velocity` (`KismetMathLibrary.MakeVector` _velocity_x _velocity_y) _charactermovement)
  (`self.LaunchCharacter` (`KismetMathLibrary.MakeVector` 0.0 0.0 Amount)))

(fn `MusicUpdate`
  (params (Score :type Integer))
  (bind _groundedaudio (`self.GroundedAudio`))
  (bind _vacationaudio (`self.VacationAudio`))
  (bind _bouncingaudio (`self.BouncingAudio`))
  (if (> Score 100)
    (if (not (`AudioComponent.IsPlaying` _vacationaudio))
      (`AudioComponent.Play` _vacationaudio 0.0)
      (`AudioComponent.AdjustVolume` _vacationaudio 0.0 (`/Game/BluePrints/BalloonGameInstance.MusicSetting` (`self.Game Instance`)) "Linear")
      (`AudioComponent.Stop` (`self.BouncingAudio`))
      (`AudioComponent.Stop` (`self.GroundedAudio`)))
    (elif (> Score 50)
      (if (not (`AudioComponent.IsPlaying` _bouncingaudio))
        (`AudioComponent.Play` _bouncingaudio (`self.Song Start`))
        (`AudioComponent.AdjustVolume` _bouncingaudio 0.0 (`/Game/BluePrints/BalloonGameInstance.MusicSetting` (`self.Game Instance`)) "Linear")
        (`AudioComponent.Stop` (`self.VacationAudio`))
        (`AudioComponent.Stop` (`self.GroundedAudio`)))
      (elif (not (`AudioComponent.IsPlaying` _groundedaudio))
        (`AudioComponent.Play` _groundedaudio (`self.Song Start`))
        (`AudioComponent.AdjustVolume` _groundedaudio 0.0 (`/Game/BluePrints/BalloonGameInstance.MusicSetting` (`self.Game Instance`)) "Linear")
        (`AudioComponent.Stop` (`self.VacationAudio`))
        (`AudioComponent.Stop` (`self.BouncingAudio`))))))

(fn `SetUpAudio`
  (`|ExecutionSequence`
    (:`then_0`
      (bind _returnvalue (`AddComponent|NODE_AddAudioComponent-5`))
      (bind _output_get (set `self.GroundedAudio` _returnvalue))
      (`AudioComponent.Play` _output_get 0.0)
      (`AudioComponent.AdjustVolume` _output_get (`/Game/BluePrints/BalloonGameInstance.MusicSetting` (`self.Game Instance`)) 1.0 "Linear"))
    (:`then_1`
      (bind _returnvalue_2 (`AddComponent|NODE_AddAudioComponent-6`))
      (bind _output_get_2 (set `self.BouncingAudio` _returnvalue_2))
      (`AudioComponent.Play` _output_get_2 0.0)
      (`AudioComponent.AdjustVolume` _output_get_2 0.0 0.0 "Linear"))
    (:`then_2`
      (bind _returnvalue_3 (`AddComponent|NODE_AddAudioComponent-7`))
      (bind _output_get_3 (set `self.VacationAudio` _returnvalue_3))
      (`AudioComponent.Play` _output_get_3 0.0)
      (`AudioComponent.AdjustVolume` _output_get_3 0.0 0.0 "Linear"))))

(fn `SetUpUI`
  (bind _returnvalue (`|CreateWidget` "/Game/UI/Score_HUD.Score_HUD_C"))
  (`UserWidget.AddToViewport` _returnvalue 0)
  (bind _output_get (set `self.UI Reference` _returnvalue))
  (`/Game/BluePrints/BP_BaseGun.SetUIReference` (`self.EquippedGun`) _output_get)
  (bind _returnvalue_2 (`|CreateWidget` "/Game/UI/PauseMenu.PauseMenu_C"))
  (bind _output_get_2 (set `self.Pause Menu` _returnvalue_2))
  (`UserWidget.AddToViewport` _output_get_2 0)
  (`Widget.SetVisibility` _output_get_2 "Hidden"))

(fn `SetUpWeapon`
  (bind _returnvalue (`|SpawnActorFromClass` "/Game/BluePrints/BP_Pistol.BP_Pistol_C" (`KismetMathLibrary.MakeTransform` (0.0 0.0 0.0)) "Undefined" "OverrideRootScale" null null))
  (bind _output_get (set `self.EquippedGun` _returnvalue))
  (`self.K2_AttachToComponent` _output_get (`self.GunLocation`) "None" "KeepRelative" "KeepRelative" "KeepRelative" true))

(fn `UserConstructionScript`)