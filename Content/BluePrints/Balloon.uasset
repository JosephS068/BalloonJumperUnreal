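; Balloon actor that drifts vertically each tick by a FallSpeed-based offset and can be popped by being shot or jumped on.
; SetConfiguration applies size, material, fall speed, scores and jump force from a configuration struct.
; JumpedOn and Shot play pop sounds, increment the GameInstance's popped count and return score, plus bounce amount for jumps.
; Pops and tail-to-Floor overlaps call Died, which spawns a DeadBalloon above and destroys the actor.
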(event `self.ReceiveBeginPlay`
  (bind _asballoon_game_instance (cast `/Game/BluePrints/BalloonGameInstance` (`GameplayStatics.GetGameInstance`)))
  (set `self.Balloon Game Instance` _asballoon_game_instance))

(event `self.ReceiveTick`
  (params (DeltaSeconds :type "Float (single-precision)"))
  (bind _output_get (set `self.Zvalue` (* (+ (`self.Zvalue`) (`self.Fall Speed`)) DeltaSeconds)))
  (`self.K2_AddActorWorldOffset` (`KismetMathLibrary.MakeVector` 0.0 0.0 _output_get)))

(event `self.Tail-Floor Collision.OnComponentBeginOverlap`
  (params (OverlappedComponent :type "PrimitiveComponent Object Reference") (OtherActor :type "Actor Object Reference") (OtherComp :type "PrimitiveComponent Object Reference") (OtherBodyIndex :type Integer) (bFromSweep :type Boolean) (SweepResult :type "HitResult Structure (by ref)"))
  (cast `/Game/BluePrints/Floor` OtherActor)
  (`self.Died`)
  (`GameplayStatics.PlaySoundAtLocation` "/Game/Sound/soft-balloon_low.soft-balloon_low" (`self.K2_GetActorLocation`) (struct) 1.0 1.0 0.0 null null null null))

(fn `DestroyTheBalloon`
  ;[1 1 1] Originally created for if destroying the balloon needed anything special handling
  (`self.K2_DestroyActor`))

(fn `Died`
  (`|SpawnActorFromClass` "/Game/BluePrints/DeadBalloon.DeadBalloon_C" (`KismetMathLibrary.Conv_VectorToTransform` (+ (`self.K2_GetActorLocation`) (0.0 0.0 150.0))) "Undefined" "OverrideRootScale" null null)
  (`self.DestroyTheBalloon`))

(fn `JumpedOn`
  (returns (ScoreValue :type Integer) (JumpAmount :type "Float (double-precision)"))
  (`GameplayStatics.PlaySoundAtLocation` "/Game/Sound/soft-balloon-pop-88692.soft-balloon-pop-88692" (`self.K2_GetActorLocation`) (struct) 1.0 1.0 0.0 null null null null)
  (`self.Died`)
  (`/Game/BluePrints/BalloonGameInstance.IncrementBalloonsPopped` (`self.Balloon Game Instance`))
  (return (`self.Jump Score`) (`self.Jump Amount`)))

(fn `Set Configuration`
  (params (`Balloon Configuration` :type "/Game/Structs/Balloon_Configuration Structure"))
  (bind (_returnvalue_location _returnvalue_rotation) (`KismetMathLibrary.BreakTransform` (`self.GetTransform`)))
  (set `self.Shot Score` `Balloon Configuration_ShotScore_4_CFC5E37B44ADC2625C3D419AA7A48452`)
  (set `self.Jump Score` `Balloon Configuration_JumpScore_5_DED5ABA54F535DC5DF6EB69150A976AF`)
  (`self.K2_SetActorTransform` (`KismetMathLibrary.MakeTransform` _returnvalue_location _returnvalue_rotation (`KismetMathLibrary.MakeVector` `Balloon Configuration_Width_11_C38D719F4C4F4A64DAC9A2B36BB85ECB` `Balloon Configuration_Width_11_C38D719F4C4F4A64DAC9A2B36BB85ECB` `Balloon Configuration_Height_10_F6ECD0824AC863F9E9A704AD85499D2B`)))
  (`PrimitiveComponent.SetMaterial` (`self.Tail-Floor Collision`) 0 `Balloon Configuration_Material_14_29D563C24AC2A016CC7FFF92491C81D1`)
  (`PrimitiveComponent.SetMaterial` (`self.Body`) 0 `Balloon Configuration_Material_14_29D563C24AC2A016CC7FFF92491C81D1`)
  (set `self.Jump Amount` `Balloon Configuration_JumpForce_17_AA3B4180406B94B1861A57BC954C3506`)
  (set `self.Fall Speed` `Balloon Configuration_FallSpeed_19_018D0D5443CC60339951CF8671C86C52`))

(fn `Shot`
  (returns (Score :type Integer))
  (`GameplayStatics.PlaySoundAtLocation` "/Game/Sound/pop-94319.pop-94319" (`self.K2_GetActorLocation`) (struct) 1.0 1.0 0.0 null null null null)
  (`self.Died`)
  (`/Game/BluePrints/BalloonGameInstance.IncrementBalloonsPopped` (`self.Balloon Game Instance`))
  (return (`self.Shot Score`)))

(fn `UserConstructionScript`)