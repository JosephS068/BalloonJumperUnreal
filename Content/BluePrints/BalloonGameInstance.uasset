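; Game instance for a balloon game that holds persistent player stats, namely balloons popped and high score, and saves them to a slot.
; Init loads the stats from the save slot if one exists.
; SaveGame loads or creates a BalloonSaveGame, copies the stats into it and writes it back.
; Helper functions increment the popped count and raise the high score only when beaten, without saving by themselves.
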(event `Save Game`
  (bind _savegamename (`self.SaveGameName`))
  (bind _returnvalue (`GameplayStatics.DoesSaveGameExist` _savegamename))
  (if _returnvalue
    (bind _returnvalue_2 (`GameplayStatics.LoadGameFromSlot` _savegamename))
    (bind _asballoon_save_game (cast `/Game/BluePrints/BalloonSaveGame` _returnvalue_2))
    (set `self.BalloonSaveGame` _asballoon_save_game)
    (else
      (bind _returnvalue_3 (`GameplayStatics.CreateSaveGameObject` "/Game/BluePrints/BalloonSaveGame.BalloonSaveGame_C"))
      (set `self.BalloonSaveGame` _returnvalue_3)))
  (set `/Game/BluePrints/BalloonSaveGame.Stats` (`self.GameStats`) (`self.BalloonSaveGame`))
  (`GameplayStatics.SaveGameToSlot` (`self.BalloonSaveGame`) (`self.SaveGameName`)))

(event `Load Game`
  (bind _savegamename (`self.SaveGameName`))
  (bind _returnvalue (`GameplayStatics.DoesSaveGameExist` _savegamename))
  (if _returnvalue
    (bind _returnvalue_2 (`GameplayStatics.LoadGameFromSlot` _savegamename))
    (bind _asballoon_save_game (cast `/Game/BluePrints/BalloonSaveGame` _returnvalue_2))
    (bind _output_get (set `self.BalloonSaveGame` _asballoon_save_game))
    (set `self.GameStats` (`/Game/BluePrints/BalloonSaveGame.Stats` _output_get))))

(event `self.ReceiveInit`
  (`self.Load Game`))

(fn `AttemptToSetHighScore`
  (params (PossibleHighScore :type Integer))
  (bind (_gamestats_balloonspopped _gamestats_highscore) (break `/Game/Structs/Records_Struct` (`self.GameStats`)))
  (if (> PossibleHighScore _gamestats_highscore)
    (set `self.GameStats` (make `/Game/Structs/Records_Struct` _gamestats_balloonspopped PossibleHighScore))))

(fn `IncrementBalloonsPopped`
  (bind (_gamestats_balloonspopped _gamestats_highscore) (break `/Game/Structs/Records_Struct` (`self.GameStats`)))
  (bind _result (`/Engine/EditorBlueprintResources/StandardMacros.IncrementInt` _gamestats_balloonspopped)
    (:`  `
      (set `self.GameStats` (make `/Game/Structs/Records_Struct` _result _gamestats_highscore)))))