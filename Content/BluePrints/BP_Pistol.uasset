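; BP_Pistol is a child weapon Blueprint for a balloon-shooting game that scores hits through a UI reference.
; Shoot calls its parent, plays gunshot sound, emitter and Niagara effects via HandleGunEffects, then runs a multi line trace on Visibility out to FireDistance.
; When the trace reports a hit, it loops over the results, calls Shot on actors that cast to Balloon and passes the returned value to AddToScore.
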(fn `HandleGunEffects`
  (bind _relativelocation (`SceneComponent.RelativeLocation` (`self.SmokeLocation`)))
  (`GameplayStatics.PlaySoundAtLocation` "/Game/Sound/Gunshot.Gunshot" (`self.K2_GetActorLocation`) (struct) 1.0 1.0 0.0 null null null null)
  (`GameplayStatics.SpawnEmitterAtLocation` null _relativelocation)
  (`AddComponent|NODE_AddNiagaraComponent-5` :`RelativeTransform` (`KismetMathLibrary.Conv_VectorToTransform` _relativelocation)))

(fn `Shoot`
  (params (StartLocation :type "Vector Structure") (ForwardVector :type "Vector Structure"))
  (`parent.Shoot` StartLocation ForwardVector)
  (`self.HandleGunEffects`)
  (bind (_outhits _returnvalue) (`KismetSystemLibrary.LineTraceMulti` StartLocation (+ StartLocation (* ForwardVector (`self.FireDistance`))) "TraceTypeQuery1"))
  (if _returnvalue
    (for _array_element _outhits
      (bind _asballoon (cast `/Game/BluePrints/Balloon` (`.HitActor` (`GameplayStatics.BreakHitResult` _array_element))))
      (bind _score (`/Game/BluePrints/Balloon.Shot` _asballoon))
      (`/Game/UI/Score_HUD.AddToScore` (`self.UI Reference`) _score))))

(fn `UserConstructionScript`
  (`parent.UserConstructionScript`))